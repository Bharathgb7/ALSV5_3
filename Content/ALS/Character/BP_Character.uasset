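; Player character for an ALS-style locomotion setup, handling Enhanced Input movement, look, jump, crouch and weapon switching.
; Aim and crouch set a gait through UpdateGate, which applies per-gait movement settings and notifies the anim instance.
; Weapon switching links Unarmed, Pistol or Rifle anim layers and re-attaches guns to sockets.
; Tick sphere-traces ground distance for the anim instance; K and L toggle debug slow motion.
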(event `EnhancedInput|/Game/ALS/Input/InputActions/IA_Aim`
  (params (ActionValue :type Boolean) (ElapsedSeconds :type "Float (double-precision)") (TriggeredSeconds :type "Float (double-precision)") (InputAction :type "InputAction Object Reference" :default "/Game/ALS/Input/InputActions/IA_Aim.IA_Aim"))
  ;[1 0.6791 0] Deciding Which State To Carry While Aiming
  (:`Started`
    (`self.UpdateGate` "NewEnumerator0"))
  (:`Completed`
    (`self.UpdateGate` "NewEnumerator1")))

(event `self.ReceiveBeginPlay`
  ;[1 0.6791 0] Setting Up Enhanced I/P for Weapon Switching and linking animation BP's
  (bind _asplayer_controller (cast `PlayerController` (`self.GetController`)))
  (message `EnhancedInputSubsystemInterface.AddMappingContext` (pcsubsystem `EnhancedInputLocalPlayerSubsystem` _asplayer_controller) "/Game/ALS/Input/IMC_ALS.IMC_ALS" 0 (struct))
  (`SkeletalMeshComponent.LinkAnimClassLayers` (`self.Mesh`) "/Game/ALS/Animation/Blueprints/ABP_Layers.ABP_Layers_C"))

(event `EnhancedInput|/Game/ALS/Input/InputActions/IA_LookAction`
  (params (ActionValue :type "Vector2D Structure") (ElapsedSeconds :type "Float (double-precision)") (TriggeredSeconds :type "Float (double-precision)") (InputAction :type "InputAction Object Reference" :default "/Game/ALS/Input/InputActions/IA_LookAction.IA_LookAction"))
  (bind (_x _y) (`KismetMathLibrary.BreakVector2D` ActionValue))
  ;[1 0.6791 0] Looking Around Using Mouse
  (:`Triggered`
    (`self.AddControllerYawInput` _x)
    (`self.AddControllerPitchInput` _y)))

(event `EnhancedInput|/Game/ALS/Input/InputActions/IA_SwitchWeapon`
  (params (ActionValue :type "Float (double-precision)") (ElapsedSeconds :type "Float (double-precision)") (TriggeredSeconds :type "Float (double-precision)") (InputAction :type "InputAction Object Reference" :default "/Game/ALS/Input/InputActions/IA_SwitchWeapon.IA_SwitchWeapon"))
  ;[0 1 0.6725] Switching Weapon Based On Enums and Playing the Respective Anim Class
  (:`Started`
    (switch `int` (`KismetMathLibrary.FTrunc` ActionValue)
      (:`1`
        (set `self.EquippedGuns` "NewEnumerator0")
        (`SkeletalMeshComponent.LinkAnimClassLayers` (`self.Mesh`) "/Game/ALS/Animation/Blueprints/ABP_Unarmed.ABP_Unarmed_C"))
      (:`2`
        (set `self.EquippedGuns` "NewEnumerator1")
        (`SkeletalMeshComponent.LinkAnimClassLayers` (`self.Mesh`) "/Game/ALS/Animation/Blueprints/ABP_Pistol.ABP_Pistol_C"))
      (:`3`
        (set `self.EquippedGuns` "NewEnumerator2")
        (`SkeletalMeshComponent.LinkAnimClassLayers` (`self.Mesh`) "/Game/ALS/Animation/Blueprints/ABP_Rifle.ABP_Rifle_C")))
    (`self.ChangeWeapon`)))

(event `Key|K`
  (params (Key :type "Key Structure"))
  ;[0 1 0.6725] Slomo on PIE
  (:`Pressed`
    (`GameplayStatics.SetGlobalTimeDilation` 0.2)))

(event `Key|L`
  (params (Key :type "Key Structure"))
  ;[0 1 0.6725] Slomo on PIE
  (:`Pressed`
    (`GameplayStatics.SetGlobalTimeDilation` 1.0)))

(event `EnhancedInput|/Game/ALS/Input/InputActions/IA_Move`
  (params (ActionValue :type "Vector2D Structure") (ElapsedSeconds :type "Float (double-precision)") (TriggeredSeconds :type "Float (double-precision)") (InputAction :type "InputAction Object Reference" :default "/Game/ALS/Input/InputActions/IA_Move.IA_Move"))
  (bind (_x _y) (`KismetMathLibrary.BreakVector2D` ActionValue))
  (bind (_returnvalue_roll _returnvalue_pitch _returnvalue_yaw) (`KismetMathLibrary.BreakRotator` (`self.GetControlRotation`)))
  (bind (_returnvalue_roll_2 _returnvalue_pitch_2 _returnvalue_yaw_2) (`KismetMathLibrary.BreakRotator` (`self.GetControlRotation`)))
  ;[1 0.6791 0] Moving Around With Keyboard
  (:`Triggered`
    ;;[0 0.1402 1] For Left and Right Movement
    (`self.AddMovementInput` (`KismetMathLibrary.GetRightVector` (`KismetMathLibrary.MakeRotator` _returnvalue_roll 0.0 _returnvalue_yaw)) _x)
    ;;[0 0.1402 1] For Forward and Backward Movement
    (`self.AddMovementInput` (`KismetMathLibrary.GetForwardVector` (`KismetMathLibrary.MakeRotator` 0.0 0.0 _returnvalue_yaw_2)) _y)))

(event `EnhancedInput|/Game/ALS/Input/InputActions/IA_Crouch`
  (params (ActionValue :type Boolean) (ElapsedSeconds :type "Float (double-precision)") (TriggeredSeconds :type "Float (double-precision)") (InputAction :type "InputAction Object Reference" :default "/Game/ALS/Input/InputActions/IA_Crouch.IA_Crouch"))
  ;[0.9294 1 0] Crouch Action
  (:`Started`
    (switch `/Game/ALS/Enums/E_Gate` (`self.CurrentGate`)
      (:`NewEnumerator0`
        (`self.UpdateGate` "NewEnumerator2" :!label _label)
        (`self.Crouch`))
      (:`NewEnumerator1`
        (goto _label))
      (:`NewEnumerator2`
        (`self.UpdateGate` "NewEnumerator1")
        (`self.UnCrouch`)))))

(event `EnhancedInput|/Game/ALS/Input/InputActions/IA_Jump`
  (params (ActionValue :type Boolean) (ElapsedSeconds :type "Float (double-precision)") (TriggeredSeconds :type "Float (double-precision)") (InputAction :type "InputAction Object Reference" :default "/Game/ALS/Input/InputActions/IA_Jump.IA_Jump"))
  ;[0.9294 1 0] Jump Action
  (:`Started`
    (`self.Jump`))
  (:`Completed`
    (`self.StopJumping`)))

(event `self.ReceiveTick`
  (params (DeltaSeconds :type "Float (single-precision)"))
  ;[1 0.6791 0] Using Sphere Trace to find the ground distance with air when jumping
  (bind (_outhit _returnvalue) (`KismetSystemLibrary.SphereTraceSingle` (- (`self.K2_GetActorLocation`) (`KismetMathLibrary.MakeVector` 0.0 0.0 (`CapsuleComponent.CapsuleHalfHeight` (`self.CapsuleComponent`)))) (- (`self.K2_GetActorLocation`) (0.0 0.0 1000.0)) 5.0 "TraceTypeQuery1"))
  (if _returnvalue
    ;;[0 0.1402 1] Getting Value To ABP_Base
    (message `/Game/ALS/Interface/BPI_AnimationBlueprintInterface.RecieveGroundDistance` (`SkeletalMeshComponent.GetAnimInstance` (`self.Mesh`)) (`.Distance` (`GameplayStatics.BreakHitResult` _outhit)))))

(fn `ChangeWeapon`
  (locals (WeaponSocketNames :type "/Game/ALS/Struct/S_Sockets Structure"))
  ;[0.9294 1 0] Attaching The Type Of Weapon To Our Hand Accoding to our Key Press
  (switch `/Game/ALS/Enums/E_Guns` (`self.EquippedGuns`)
    (:`NewEnumerator0`
      (`SceneComponent.K2_AttachToComponent` (`self.Pistol`) (`self.Mesh`) (`.PistolUnEquipped_2_CD00D0604CA040EB6F7D0AB2AE69D302` (break `/Game/ALS/Struct/S_Sockets` (`local.WeaponSocketNames`))) "SnapToTarget" "SnapToTarget" "SnapToTarget" true)
      (`SceneComponent.K2_AttachToComponent` (`self.Rifle`) (`self.Mesh`) (`.PistolUnEquipped_2_CD00D0604CA040EB6F7D0AB2AE69D302` (break `/Game/ALS/Struct/S_Sockets` (`local.WeaponSocketNames`))) "SnapToTarget" "SnapToTarget" "SnapToTarget" true))
    (:`NewEnumerator1`
      (`SceneComponent.K2_AttachToComponent` (`self.Pistol`) (`self.Mesh`) (`.WeaponEquipped_6_9B10D33D41556D87DD2EE99C1BF9BFFC` (break `/Game/ALS/Struct/S_Sockets` (`local.WeaponSocketNames`))) "SnapToTarget" "SnapToTarget" "SnapToTarget" true)
      (`SceneComponent.K2_AttachToComponent` (`self.Rifle`) (`self.Mesh`) (`.RifleUnEquipped_4_A12697C94A26426B3BA4D1B53F4A76E7` (break `/Game/ALS/Struct/S_Sockets` (`local.WeaponSocketNames`))) "SnapToTarget" "SnapToTarget" "SnapToTarget" true))
    (:`NewEnumerator2`
      (`SceneComponent.K2_AttachToComponent` (`self.Pistol`) (`self.Mesh`) (`.PistolUnEquipped_2_CD00D0604CA040EB6F7D0AB2AE69D302` (break `/Game/ALS/Struct/S_Sockets` (`local.WeaponSocketNames`))) "SnapToTarget" "SnapToTarget" "SnapToTarget" true)
      (`SceneComponent.K2_AttachToComponent` (`self.Rifle`) (`self.Mesh`) (`.WeaponEquipped_6_9B10D33D41556D87DD2EE99C1BF9BFFC` (break `/Game/ALS/Struct/S_Sockets` (`local.WeaponSocketNames`))) "SnapToTarget" "SnapToTarget" "SnapToTarget" true))))

(fn `UpdateGate`
  (params (Gate :type "/Game/ALS/Enums/E_Gate Enum" :default "NewEnumerator0"))
  (bind _charactermovement (`self.CharacterMovement`))
  (bind (_maxwalkspeed _maxacceleration _brakingdeceleration _brakingfrictionfactor _brakingfriction _useseperatebrakingfriction) (break `/Game/ALS/Struct/S_GateSetting` (`BlueprintMapLibrary.Map_Find` (`self.GateSetting`) Gate)))
  (set `self.CurrentGate` Gate)
  (message `/Game/ALS/Interface/BPI_AnimationBlueprintInterface.RecieveCurrentGate` (`SkeletalMeshComponent.GetAnimInstance` (`self.Mesh`)) Gate)
  (`|ExecutionSequence`
    (:`then_0`
      (set `CharacterMovementComponent.MaxWalkSpeed` _maxwalkspeed _charactermovement))
    (:`then_1`
      (set `CharacterMovementComponent.MaxAcceleration` _maxacceleration _charactermovement))
    (:`then_2`
      (set `CharacterMovementComponent.BrakingDecelerationWalking` _brakingdeceleration _charactermovement))
    (:`then_3`
      (set `CharacterMovementComponent.BrakingFrictionFactor` _brakingfrictionfactor _charactermovement))
    (:`then_4`
      (set `CharacterMovementComponent.BrakingFriction` _brakingfriction _charactermovement))
    (:`then_5`
      (set `CharacterMovementComponent.bUseSeparateBrakingFriction` _useseperatebrakingfriction _charactermovement))))

(fn `UserConstructionScript`)